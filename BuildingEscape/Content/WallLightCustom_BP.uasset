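; Customizable wall light that reacts to the number and mass of actors inside a trigger volume.
; Construction applies the configured brightness, color and cone angles.
; Each entry scales intensity by overlap count and adds the actor's first-primitive mass, blending color from red toward green, solid green at the threshold.
; Exits subtract mass without updating intensity, until an empty volume restores the configured color and a hardcoded intensity.
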(event `self.TriggerVolume.OnActorBeginOverlap`
  (params (OverlappedActor :type "Actor Object Reference") (OtherActor :type "Actor Object Reference"))
  (bind _treshold (`self.Treshold`))
  (bind _pointlight2 (`self.PointLight2`))
  (`LightComponent.SetIntensity` _pointlight2 (* (`KismetArrayLibrary.Array_Length` (`self.GetOverlappingActors` (`self.TriggerVolume`) null)) 2000.0))
  (bind _output_get (set `self.TotalMass` (+ (`self.TotalMass`) (`PrimitiveComponent.GetMass` (`KismetArrayLibrary.Array_Get` (`self.K2_GetComponentsByClass` OtherActor "/Script/Engine.PrimitiveComponent"))))))
  (`/Engine/EditorBlueprintResources/StandardMacros.CompareFloat` _output_get _treshold
    (:`>`
      (`LightComponent.SetLightColor` _pointlight2 (struct :`G` 1.0 :`A` 1.0) true :!label _label))
    (:`==`
      (goto _label))
    (:`<`
      (bind _returnvalue (/ _output_get _treshold))
      (`LightComponent.SetLightColor` _pointlight2 (`KismetMathLibrary.MakeColor` (- 1.0 _returnvalue) _returnvalue) true))))

(event `self.TriggerVolume.OnActorEndOverlap`
  (params (OverlappedActor :type "Actor Object Reference") (OtherActor :type "Actor Object Reference"))
  (bind _treshold (`self.Treshold`))
  (bind _pointlight2 (`self.PointLight2`))
  (`/Engine/EditorBlueprintResources/StandardMacros.CompareInt` (`KismetArrayLibrary.Array_Length` (`self.GetOverlappingActors` (`self.TriggerVolume`) null))
    (:`>`
      (bind _output_get (set `self.TotalMass` (- (`self.TotalMass`) (`PrimitiveComponent.GetMass` (`KismetArrayLibrary.Array_Get` (`self.K2_GetComponentsByClass` OtherActor "/Script/Engine.PrimitiveComponent"))))))
      (`/Engine/EditorBlueprintResources/StandardMacros.CompareFloat` _output_get _treshold
        (:`>`
          (goto _label))
        (:`==`
          (goto _label))
        (:`<`
          (bind _returnvalue (/ _output_get _treshold))
          (`LightComponent.SetLightColor` _pointlight2 (`KismetMathLibrary.MakeColor` (- 1.0 _returnvalue) _returnvalue) true))))
    (:`==`
      (`LightComponent.SetIntensity` _pointlight2 666.0 :!label _label_2)
      (set `self.TotalMass` 0.0)
      (`LightComponent.SetLightColor` _pointlight2 (`self.Color`) true))
    (:`<`
      (goto _label_2))))

(fn `UserConstructionScript`
  (bind _pointlight2 (`self.PointLight2`))
  (`LightComponent.SetIntensity` _pointlight2 (`self.Brightness`))
  (`LightComponent.SetLightColor` _pointlight2 (`self.Color`) true)
  (`SpotLightComponent.SetInnerConeAngle` _pointlight2 (`self.Inner Cone Angle`))
  (`SpotLightComponent.SetOuterConeAngle` _pointlight2 (`self.Outer Cone Angle`))
  (set `self.TotalMass` 0.0))