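; Openable door actor that swings on open and close requests from its OpenDoor component.
; An open request plays a lock sound and runs the DoorSwing timeline forward; a close request reverses it.
; The timeline's yaw curve is combined with the rotation cached in the construction script to rotate the whole actor.
; Paired DoOnce gates, each reset by the opposite request, ignore repeated requests.
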(event `self.OpenDoor.OnOpenRequest`
  (`|ExecutionSequence`
    (:`then_0`
      (goto _label_3 :!via `Reset`))
    (:`then_1`
      (`/Engine/EditorBlueprintResources/StandardMacros.DoOnce` false :!label _label
        (:`Completed`
          (`GameplayStatics.PlaySoundAtLocation` "/Game/Audio/door-lock.door-lock" (`self.K2_GetActorLocation`) (struct) 0.25 0.88)
          (bind (_direction _opendoor) (`Timeline|Door Swing` :`NewTime` 2.0 :!label _label_2)
            (:`Update`
              (`self.K2_SetActorRotation` (`KismetMathLibrary.ComposeRotators` (`KismetMathLibrary.MakeRotator` 0.0 0.0 _opendoor) (`self.DoorRotation`))))))))))

(event `self.OpenDoor.OnCloseRequest`
  (`|ExecutionSequence`
    (:`then_0`
      (goto _label :!via `Reset`))
    (:`then_1`
      (`/Engine/EditorBlueprintResources/StandardMacros.DoOnce` false :!label _label_3
        (:`Completed`
          (goto _label_2 :!via `Reverse`))))))

(fn `UserConstructionScript`
  (set `self.DoorRotation` (`self.K2_GetActorRotation` (`ActorComponent.GetOwner` (`self.OpenDoor`)))))